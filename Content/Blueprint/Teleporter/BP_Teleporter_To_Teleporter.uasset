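; BP_Teleporter_To_Teleporter is a teleporter actor that sends the player to a linked receiver teleporter.
; When BP_Player overlaps its Box, the player teleports to the world location of TeleporterReceiver's PointLight, with rotation set to zero.
; The construction script tints its own PointLight with LightColor.
; A one-second collision-disable cooldown exists in the graph but is unconnected and never runs.
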(event OnComponentBeginOverlap(Box)
  (params (OverlappedComponent :type Primitive%20Component%20Object%20Reference) (OtherActor :type Actor%20Object%20Reference) (OtherComp :type Primitive%20Component%20Object%20Reference) (OtherBodyIndex :type Integer) (bFromSweep :type Boolean) (SweepResult :type Hit%20Result%20Structure%20%28by%20ref%29))
  (bind _asbp_player (Utilities|Casting|CastToBP_Player OtherActor))
  (Transformation|Teleport _asbp_player (Transformation|GetWorldLocation (Variables|/Game/Blueprint/Teleporter/BP_Teleporter_Receiver.BP_Teleporter_Receiver_C|GetPointLight (Variables|Default|GetTeleporterReceiver))) "0, 0, 0"))

(event EventBeginPlay)

(event Collision|EventActorBeginOverlap
  (params (OtherActor :type Actor%20Object%20Reference)))

(event EventTick
  (params (DeltaSeconds :type Float%20%28single-precision%29)))

(fn ConstructionScript
  (Rendering|Components|Light|SetLightColor (Variables|Default|GetPointLight) (Variables|Default|GetLightColor) true))