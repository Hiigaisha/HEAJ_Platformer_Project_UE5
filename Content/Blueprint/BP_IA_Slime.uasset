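; BP_IA_Slime is an enemy slime AI that chases the player and can be killed on contact with its interact box.
; Pawn sensing triggers AIMoveTo toward the player while the slime is alive.
; Overlapping InteractBox launches the player upward once, sets IsDead and plays a death montage before destroying the slime.
; Overlapping HitAttack_Box ragdolls the player, then respawns them after a delay, regardless of IsDead.
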(event OnSeePawn(PawnSensing)
  (params (Pawn :type Pawn%20Object%20Reference))
  ;[1 1 1] IA Follow Player
  (bind _asbp_player (Utilities|Casting|CastToBP_Player Pawn))
  (Development|PrintString "As Seen Player")
  (if (not (Variables|Default|GetisDead?))
    (AI|AIMoveTo self (Transformation|GetWorldLocation (Variables|/Script/Engine.Character|GetMesh _asbp_player)) _asbp_player 5.0 false)))

(event OnComponentBeginOverlap(InteractBox)
  (params (OverlappedComponent :type Primitive%20Component%20Object%20Reference) (OtherActor :type Actor%20Object%20Reference) (OtherComp :type Primitive%20Component%20Object%20Reference) (OtherBodyIndex :type Integer) (bFromSweep :type Boolean) (SweepResult :type Hit%20Result%20Structure%20%28by%20ref%29))
  ;[1 1 1] Kill IA
  (bind _asbp_player (Utilities|Casting|CastToBP_Player OtherActor))
  (Utilities|FlowControl|DoOnce false
    (:Completed
      (Development|PrintString "Kill IA")
      (Variables|Default|SetisDead? true)
      (Character|LaunchCharacter _asbp_player "0.000000,0.000000,750.000000" false false)
      (Animation|Montage|PlayMontage (Variables|Character|GetMesh) "/Game/Fab/MonsterForSurvivalGame/Animation/PBR/Slime/AM_Slime_Die.AM_Slime_Die"
        (:OnCompleted
          (Actor|DestroyActor))))))

(event OnComponentBeginOverlap(HitAttack_Box)
  (params (OverlappedComponent :type Primitive%20Component%20Object%20Reference) (OtherActor :type Actor%20Object%20Reference) (OtherComp :type Primitive%20Component%20Object%20Reference) (OtherBodyIndex :type Integer) (bFromSweep :type Boolean) (SweepResult :type Hit%20Result%20Structure%20%28by%20ref%29))
  (bind _asbp_player (Utilities|Casting|CastToBP_Player OtherActor))
  (if (Variables|Default|GetisDead?)
    _
    (else
      _))
  (Development|PrintString "Player Damage")
  (Default|EventRagdoll _asbp_player)
  (Utilities|FlowControl|Delay 2.0)
  (Default|EventRespawn _asbp_player))

(fn ConstructionScript)