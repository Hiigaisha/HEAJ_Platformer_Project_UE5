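; Base interactable actor that shows an on-screen message when the player comes within range.
; A Sphere overlap with BP_Player creates a UI_Message widget with MSG and ItemName joined as its text, and removes it on end overlap.
; The Interact event only prints ItemName, and the construction script applies the Mesh variable to the static mesh component.
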(event OnComponentBeginOverlap(Sphere)
  (params (OverlappedComponent :type Primitive%20Component%20Object%20Reference) (OtherActor :type Actor%20Object%20Reference) (OtherComp :type Primitive%20Component%20Object%20Reference) (OtherBodyIndex :type Integer) (bFromSweep :type Boolean) (SweepResult :type Hit%20Result%20Structure%20%28by%20ref%29))
  (Utilities|Casting|CastToBP_Player OtherActor)
  (bind _returnvalue (UserInterface|CreateWidget "/Game/Blueprint/UI/UI_Message.UI_Message_C"))
  (UserInterface|Viewport|AddtoViewport _returnvalue 0)
  (Rendering|Components|TextRender|SetText (Variables|/Game/Blueprint/UI/UI_Message.UI_Message_C|GetMSG _returnvalue) (Utilities|Text|ToText(String) (Utilities|String|Append (Utilities|String|ToString(Text) (Variables|Default|GetMSG)) (Variables|Customisation|GetItemName)))))

(event OnComponentEndOverlap(Sphere)
  (params (OverlappedComponent :type Primitive%20Component%20Object%20Reference) (OtherActor :type Actor%20Object%20Reference) (OtherComp :type Primitive%20Component%20Object%20Reference) (OtherBodyIndex :type Integer))
  (Utilities|Casting|CastToBP_Player OtherActor)
  (Widget|RemovefromParent (stale OnComponentBeginOverlap(Sphere) _returnvalue)))

(event EventInteract
  (Development|PrintString (Variables|Customisation|GetItemName)))

(fn ConstructionScript
  (Components|StaticMesh|SetStaticMesh (Variables|Default|GetStaticMesh) (Variables|Customisation|GetMesh)))