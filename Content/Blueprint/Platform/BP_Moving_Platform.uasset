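; BP_Moving_Platform is a platform that shuttles back and forth along a spline, starting on BeginPlay.
; A Timeline scales its output by spline length to set the mesh's world location and rotation, keeping roll and yaw but zeroing pitch.
; When the Timeline finishes, the IsReverse flag selects the Normal or Return event, flipping direction for an endless ping-pong.
; Rotation is sampled in spline local space yet applied as world rotation during movement.
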(event Custom|Event%20Normal
  (bind _staticmesh (Variables|Default|GetStaticMesh))
  (bind _spline (Variables|Default|GetSpline))
  (bind _spline_2 (Variables|Default|GetSpline))
  (bind _returnvalue (Spline|GetRotationatDistanceAlongSpline _spline_2 0.0 "Local"))
  (Variables|Default|SetIsReverse? false)
  (Transformation|SetRelativeRotation (Variables|Default|GetStaticMesh) (Math|Rotator|MakeRotator (.roll _returnvalue) 0.0 (.yaw _returnvalue)) false false)
  (bind _timing_platform (Timeline|Timeline Play)
    (:Update
      (Transformation|SetWorldLocation _staticmesh (Spline|GetLocationatDistanceAlongSpline _spline (* _timing_platform (Spline|GetSplineLength _spline)) "World") false false)
      (Transformation|SetWorldRotation _staticmesh (Math|Rotator|MakeRotator (.roll (Spline|GetRotationatDistanceAlongSpline _spline (* _timing_platform (Spline|GetSplineLength _spline)) "Local")) 0.0 (.yaw (Spline|GetRotationatDistanceAlongSpline _spline (* _timing_platform (Spline|GetSplineLength _spline)) "Local"))) false false))
    (:Finished
      (if (Variables|Default|GetIsReverse?)
        (CallFunction|EventNormal)
        (else
          (CallFunction|EventReturn))))))

(event Custom|Event%20Return
  (bind _staticmesh (Variables|Default|GetStaticMesh))
  (bind _spline (Variables|Default|GetSpline))
  (Variables|Default|SetIsReverse? true)
  (bind _timing_platform (Timeline|Timeline Reverse)
    (:Update
      (Transformation|SetWorldLocation _staticmesh (Spline|GetLocationatDistanceAlongSpline _spline (* _timing_platform (Spline|GetSplineLength _spline)) "World") false false)
      (Transformation|SetWorldRotation _staticmesh (Math|Rotator|MakeRotator (.roll (Spline|GetRotationatDistanceAlongSpline _spline (* _timing_platform (Spline|GetSplineLength _spline)) "Local")) 0.0 (.yaw (Spline|GetRotationatDistanceAlongSpline _spline (* _timing_platform (Spline|GetSplineLength _spline)) "Local"))) false false))
    (:Finished
      (if (Variables|Default|GetIsReverse?)
        (CallFunction|EventNormal)
        (else
          (CallFunction|EventReturn))))))

(event EventBeginPlay
  (bind _staticmesh (Variables|Default|GetStaticMesh))
  (bind _spline (Variables|Default|GetSpline))
  (bind _spline_2 (Variables|Default|GetSpline))
  (bind _returnvalue (Spline|GetRotationatDistanceAlongSpline _spline_2 0.0 "Local"))
  (Transformation|SetRelativeRotation (Variables|Default|GetStaticMesh) (Math|Rotator|MakeRotator (.roll _returnvalue) 0.0 (.yaw _returnvalue)) false false)
  (bind _timing_platform (Timeline|Timeline Play)
    (:Update
      (Transformation|SetWorldLocation _staticmesh (Spline|GetLocationatDistanceAlongSpline _spline (* _timing_platform (Spline|GetSplineLength _spline)) "World") false false)
      (Transformation|SetWorldRotation _staticmesh (Math|Rotator|MakeRotator (.roll (Spline|GetRotationatDistanceAlongSpline _spline (* _timing_platform (Spline|GetSplineLength _spline)) "Local")) 0.0 (.yaw (Spline|GetRotationatDistanceAlongSpline _spline (* _timing_platform (Spline|GetSplineLength _spline)) "Local"))) false false))
    (:Finished
      (if (Variables|Default|GetIsReverse?)
        (CallFunction|EventNormal)
        (else
          (CallFunction|EventReturn))))))

(fn ConstructionScript)