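; BP_Falling_Platform is a platform that drops after the player touches it and later returns to its starting position.
; A Box overlap by BP_Player starts a retriggerable delay, then enables physics simulation on the static mesh.
; Any actor ending overlap with the box starts the respawn delay, then Reset disables physics and moves the mesh to the root's location, leaving rotation untouched.
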(event OnComponentBeginOverlap(Box)
  (params (OverlappedComponent :type Primitive%20Component%20Object%20Reference) (OtherActor :type Actor%20Object%20Reference) (OtherComp :type Primitive%20Component%20Object%20Reference) (OtherBodyIndex :type Integer) (bFromSweep :type Boolean) (SweepResult :type Hit%20Result%20Structure%20%28by%20ref%29))
  (Utilities|Casting|CastToBP_Player OtherActor)
  (Utilities|FlowControl|RetriggerableDelay (Variables|Default|GetOn_Platform_Time))
  (Physics|SetSimulatePhysics (Variables|Default|GetStaticMesh) true))

(event OnComponentEndOverlap(Box)
  (params (OverlappedComponent :type Primitive%20Component%20Object%20Reference) (OtherActor :type Actor%20Object%20Reference) (OtherComp :type Primitive%20Component%20Object%20Reference) (OtherBodyIndex :type Integer))
  (Utilities|FlowControl|Delay (Variables|Default|GetRespawn_Time))
  (CallFunction|EventReset))

(event Custom|Event%20Reset
  (bind _staticmesh (Variables|Default|GetStaticMesh))
  (Physics|SetSimulatePhysics _staticmesh false)
  (Transformation|SetWorldLocation _staticmesh (Transformation|GetWorldLocation (Variables|Default|GetDefaultSceneRoot)) false false))

(fn ConstructionScript)