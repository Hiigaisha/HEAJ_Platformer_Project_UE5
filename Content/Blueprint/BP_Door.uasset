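; BP_Door is a key-locked door that the player opens and closes through an Interact event.
; It checks the BP_Player's HaveKey array at the door's WhichKeyNumber index and prints "Need Key" if that key is missing.
; With the key, a FlipFlop alternates a Timeline between playing and reversing, sliding the Door component vertically.
; Both the locked and unlocked branches play the same S_Door_Locked sound.
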(event EventInteract
  (bind _asbp_player (Utilities|Casting|CastToBP_Player (Game|GetPlayerCharacter 0)))
  (if (Utilities|Array|Get(acopy) (Variables|/Game/Character/Player/BP_Player.BP_Player_C|GetHaveKey? _asbp_player) (Variables|Default|GetWhichKeyNumber))
    (Development|PrintString "Open")
    (Audio|PlaySoundatLocation "/Game/Sounds/S_Door_Locked.S_Door_Locked" (Transformation|GetActorLocation) "0, 0, 0" 1.0 1.0 0.0 0 0 0 0)
    (Utilities|FlowControl|FlipFlop
      (:A
        (bind _newtrack_0 (Timeline|Timeline PlayFromStart)
          (:Update
            (Transformation|SetRelativeLocation (Variables|Default|GetDoor) (Math|Vector|MakeVector 0.0 0.0 (Math|Float|Lerp 1.9e+02 4.9e+02 _newtrack_0)) false false))))
      (:B
        (Timeline|Timeline Reverse)))
    (else
      (Development|PrintString "Need Key")
      (Audio|PlaySoundatLocation "/Game/Sounds/S_Door_Locked.S_Door_Locked" (Transformation|GetActorLocation) "0, 0, 0" 1.0 1.0 0.0 0 0 0 0))))

(fn ConstructionScript)